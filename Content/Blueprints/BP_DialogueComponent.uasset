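; BP_DialogueComponent is a dialogue component that shows a list of text lines one at a time in a WBP_Dialogue widget.
; On BeginPlay it creates the widget, adds it to the viewport and keeps it collapsed.
; StartDialogue resets the line index and reveals the widget, and each ShowNextDialogue call displays the next line or collapses the widget after the last.
; StopDialogue resets the index and hides the widget.
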(event `self.ReceiveBeginPlay`
  (bind _returnvalue (`|CreateWidget` "/Game/Blueprints/Widgets/WBP_Dialogue.WBP_Dialogue_C"))
  (bind _output_get (set `self.DialogueWidget` _returnvalue))
  (`UserWidget.AddToViewport` _output_get 0)
  (`Widget.SetVisibility` (`self.DialogueWidget`) "Collapsed"))

(fn `ShowNextDialogue`
  (bind _currentlineindex (`self.CurrentLineIndex`))
  (bind _dialoguelines (`self.DialogueLines`))
  (`/Engine/EditorBlueprintResources/StandardMacros.CompareInt` _currentlineindex (`KismetArrayLibrary.Array_Length` _dialoguelines)
    (:`==`
      (`Widget.SetVisibility` (`self.DialogueWidget`) "Collapsed"))
    (:`<`
      (`RichTextBlock.SetText` (`/Game/Blueprints/Widgets/WBP_Dialogue.Text_Dialogue` (`self.DialogueWidget`)) (`|GetArrayItem` _dialoguelines _currentlineindex))
      (`/Engine/EditorBlueprintResources/StandardMacros.IncrementInt` (`self.CurrentLineIndex`)))))

(fn `StartDialogue`
  (set `self.CurrentLineIndex` 0)
  (`Widget.SetVisibility` (`self.DialogueWidget`) "Visible")
  (`self.ShowNextDialogue`))

(fn `StopDialogue`
  (set `self.CurrentLineIndex` 0)
  (`Widget.SetVisibility` (`self.DialogueWidget`) "Collapsed"))